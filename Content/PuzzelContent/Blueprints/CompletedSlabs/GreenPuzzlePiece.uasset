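; Green puzzle slab that the player toggles lit or unlit with the tile interaction input while standing in its box trigger.
; Each toggle flips the material's emissive parameter, light intensity and TileActive, with a short cooldown blocking repeat presses.
; A press also briefly spawns a GreenTriggerCollision actor at the slab's transform.
; ActivatedByOtherTile performs the same toggle without spawning a trigger, apparently so other tiles can flip it.
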(event `self.ReceiveBeginPlay`
  (`self.EnableInput` (`GameplayStatics.GetPlayerController` 0)))

(event `self.Box.OnComponentBeginOverlap`
  (params (OverlappedComponent :type "PrimitiveComponent Object Reference") (OtherActor :type "Actor Object Reference") (OtherComp :type "PrimitiveComponent Object Reference") (OtherBodyIndex :type Integer) (bFromSweep :type Boolean) (SweepResult :type "HitResult Structure (by ref)"))
  (cast `/Game/ThirdPerson/Blueprints/BP_MainCharacterBase` OtherActor
    (:`then`
      (set `self.PlayerIsTouching` true))
    (:`CastFailed`
      (set `self.PlayerIsTouching` false))))

(event `self.Box.OnComponentEndOverlap`
  (params (OverlappedComponent :type "PrimitiveComponent Object Reference") (OtherActor :type "Actor Object Reference") (OtherComp :type "PrimitiveComponent Object Reference") (OtherBodyIndex :type Integer))
  (cast `/Game/ThirdPerson/Blueprints/BP_MainCharacterBase` OtherActor)
  (set `self.PlayerIsTouching` false))

(event `EnhancedInput|/Game/ThirdPerson/Input/Actions/IA_TileInteraction`
  (params (ActionValue :type Boolean) (ElapsedSeconds :type "Float (double-precision)") (TriggeredSeconds :type "Float (double-precision)") (InputAction :type "InputAction Object Reference" :default "/Game/ThirdPerson/Input/Actions/IA_TileInteraction.IA_TileInteraction"))
  (bind _emissivelight (`self.EmissiveLight`))
  (:`Triggered`
    (if (`self.PlayerIsTouching`)
      ;[1 1 1] BasicTileFunction(ClickEforLightToggle)
      (if (`self.Is Pushable`)
        (set `self.Is Pushable` false)
        (bind _returnvalue (`PrimitiveComponent.CreateDynamicMaterialInstance` (`self.GreenSlab`) 0 null "None"))
        (bind _output_get (set `self.NewTileMaterial` _returnvalue))
        (bind _returnvalue_2 (`MaterialInstanceDynamic.K2_GetScalarParameterValue` _output_get "EmissiveToggle"))
        (if (== _returnvalue_2 1.0)
          (`MaterialInstanceDynamic.SetScalarParameterValue` _output_get "EmissiveToggle" 0.0)
          (`LightComponent.SetIntensity` _emissivelight 0.0)
          (bind _returnvalue_3 (`|SpawnActorFromClass` "/Game/PuzzelContent/Blueprints/GreenTriggerCollision.GreenTriggerCollision_C" (`self.GetTransform`) "AlwaysSpawn" "OverrideRootScale" null null))
          (`KismetSystemLibrary.Delay` 0.14)
          (`self.K2_DestroyActor` _returnvalue_3)
          (`KismetSystemLibrary.Delay` 1.0)
          (set `self.Is Pushable` true)
          (set `self.TileActive` false)
          (else
            (`MaterialInstanceDynamic.SetScalarParameterValue` _output_get "EmissiveToggle" 1.0)
            (`LightComponent.SetIntensity` _emissivelight 500.0)
            (bind _returnvalue_4 (`|SpawnActorFromClass` "/Game/PuzzelContent/Blueprints/GreenTriggerCollision.GreenTriggerCollision_C" (`self.GetTransform`) "AlwaysSpawn" "OverrideRootScale" null null))
            (`KismetSystemLibrary.Delay` 0.14)
            (`self.K2_DestroyActor` _returnvalue_4)
            (`KismetSystemLibrary.Delay` 1.0)
            (set `self.Is Pushable` true)
            (set `self.TileActive` true)))))))

(fn `ActivatedByOtherTile`
  (bind _emissivelight (`self.EmissiveLight`))
  (bind _returnvalue (`PrimitiveComponent.CreateDynamicMaterialInstance` (`self.GreenSlab`) 0 null "None"))
  (bind _output_get (set `self.NewTileMaterial` _returnvalue))
  (bind _returnvalue_2 (`MaterialInstanceDynamic.K2_GetScalarParameterValue` _output_get "EmissiveToggle"))
  (if (== _returnvalue_2 1.0)
    (`MaterialInstanceDynamic.SetScalarParameterValue` _output_get "EmissiveToggle" 0.0)
    (`LightComponent.SetIntensity` _emissivelight 0.0)
    (set `self.TileActive` false)
    (else
      (`MaterialInstanceDynamic.SetScalarParameterValue` _output_get "EmissiveToggle" 1.0)
      (`LightComponent.SetIntensity` _emissivelight 500.0)
      (set `self.TileActive` true))))

(fn `UserConstructionScript`)