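; Trigger actor for a tile puzzle that activates the puzzle tiles it overlaps.
; Each of its four collision components, on begin overlap, waits its own short staggered delay and then runs CheckForTileType.
; That function queries the whole actor's overlaps by class and calls ActivatedByOtherTile on every CombinedSlab and red, blue or green puzzle piece found.
; The Delay after each check has nothing wired after it.
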(event `self.CrosshairCollision1.OnComponentBeginOverlap`
  (params (OverlappedComponent :type "PrimitiveComponent Object Reference") (OtherActor :type "Actor Object Reference") (OtherComp :type "PrimitiveComponent Object Reference") (OtherBodyIndex :type Integer) (bFromSweep :type Boolean) (SweepResult :type "HitResult Structure (by ref)"))
  (`KismetSystemLibrary.Delay` 0.4)
  (`self.Check For Tile type`)
  (`KismetSystemLibrary.Delay` 0.4))

(event `self.Box2.OnComponentBeginOverlap`
  (params (OverlappedComponent :type "PrimitiveComponent Object Reference") (OtherActor :type "Actor Object Reference") (OtherComp :type "PrimitiveComponent Object Reference") (OtherBodyIndex :type Integer) (bFromSweep :type Boolean) (SweepResult :type "HitResult Structure (by ref)"))
  (`KismetSystemLibrary.Delay` 0.2)
  (`self.Check For Tile type`)
  (`KismetSystemLibrary.Delay` 0.2))

(event `self.Box3.OnComponentBeginOverlap`
  (params (OverlappedComponent :type "PrimitiveComponent Object Reference") (OtherActor :type "Actor Object Reference") (OtherComp :type "PrimitiveComponent Object Reference") (OtherBodyIndex :type Integer) (bFromSweep :type Boolean) (SweepResult :type "HitResult Structure (by ref)"))
  (`KismetSystemLibrary.Delay` 0.3)
  (`self.Check For Tile type`)
  (`KismetSystemLibrary.Delay` 0.3))

(event `self.CrosshairCollision.OnComponentBeginOverlap`
  (params (OverlappedComponent :type "PrimitiveComponent Object Reference") (OtherActor :type "Actor Object Reference") (OtherComp :type "PrimitiveComponent Object Reference") (OtherBodyIndex :type Integer) (bFromSweep :type Boolean) (SweepResult :type "HitResult Structure (by ref)"))
  (`KismetSystemLibrary.Delay` 0.1)
  (`self.Check For Tile type`)
  (`KismetSystemLibrary.Delay` 0.1))

(fn `Check For Tile type`
  (for _array_element (`self.GetOverlappingActors` "/Game/PuzzelContent/Blueprints/CompletedSlabs/CombinedSlab.CombinedSlab_C")
    (bind _ascombined_slab (cast `/Game/PuzzelContent/Blueprints/CompletedSlabs/CombinedSlab` _array_element))
    (`/Game/PuzzelContent/Blueprints/CompletedSlabs/CombinedSlab.ActivatedByOtherTile` _ascombined_slab))
  (for _array_element_2 (`self.GetOverlappingActors` "/Game/PuzzelContent/Blueprints/CompletedSlabs/RedPuzzlePiece.RedPuzzlePiece_C")
    (bind _asred_puzzle_piece (cast `/Game/PuzzelContent/Blueprints/CompletedSlabs/RedPuzzlePiece` _array_element_2))
    (`/Game/PuzzelContent/Blueprints/CompletedSlabs/RedPuzzlePiece.ActivatedByOtherTile` _asred_puzzle_piece))
  (for _array_element_3 (`self.GetOverlappingActors` "/Game/PuzzelContent/Blueprints/CompletedSlabs/BluePuzzlePiece.BluePuzzlePiece_C")
    (bind _asblue_puzzle_piece (cast `/Game/PuzzelContent/Blueprints/CompletedSlabs/BluePuzzlePiece` _array_element_3))
    (`/Game/PuzzelContent/Blueprints/CompletedSlabs/BluePuzzlePiece.ActivatedByOtherTile` _asblue_puzzle_piece))
  (for _array_element_4 (`self.GetOverlappingActors` "/Game/PuzzelContent/Blueprints/CompletedSlabs/GreenPuzzlePiece.GreenPuzzlePiece_C")
    (bind _asgreen_puzzle_piece (cast `/Game/PuzzelContent/Blueprints/CompletedSlabs/GreenPuzzlePiece` _array_element_4))
    (`/Game/PuzzelContent/Blueprints/CompletedSlabs/GreenPuzzlePiece.ActivatedByOtherTile` _asgreen_puzzle_piece)))

(fn `UserConstructionScript`)