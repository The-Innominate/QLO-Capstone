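; Puzzle board actor that builds a grid of grey, red and blue tiles and detects when the active tiles match an answer key.
; BeginPlay spawns tiles from the GridTiles type codes, plus a tilted BP_BoardToCopy1 board nearby.
; Tick, throttled by a half-second Delay, bubble-sorts the active tile indices, then updates and compares them with AnswerKey.
; A match sets GameWon and destroys the board to copy.
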(event `self.ReceiveBeginPlay`
  (bind _returnvalue (`SceneComponent.K2_GetComponentToWorld` (`self.DefaultSceneRoot`)))
  (`self.GenerateBoard`)
  (bind _returnvalue_2 (`|SpawnActorFromClass` "/Game/PuzzelContent/Blueprints/BP_BoardToCopy1.BP_BoardToCopy1_C" (`KismetMathLibrary.MakeTransform` (`KismetMathLibrary.MakeVector` (.x (.location _returnvalue)) (+ (.y (.location _returnvalue)) 100.0) (+ (.z (.location _returnvalue)) 100.0)) (`KismetMathLibrary.MakeRotator` (.roll (.rotation _returnvalue)) -90.0 (+ (.yaw (.rotation _returnvalue)) 10.0)) (.scale _returnvalue)) "Undefined" "MultiplyWithRoot" null null)))

(event `self.ReceiveTick`
  (params (DeltaSeconds :type "Float (single-precision)"))
  (`KismetSystemLibrary.Delay` 0.5)
  (`self.SortCurrentAnwers`)
  (`self.CheckWinCondition`)
  (if (`self.GameWon`)
    (`self.K2_DestroyActor` (stale `self.ReceiveBeginPlay` _returnvalue_2))))

(fn `CheckWinCondition`
  (bind _currentanswer (`self.CurrentAnswer`))
  (bind _currentanswer_2 (`self.CurrentAnswer`))
  (for (_array_element _array_index) (`self.TileReferences`)
    (bind _ascombined_slab (cast `/Game/PuzzelContent/Blueprints/CompletedSlabs/CombinedSlab` _array_element)
      (:`then`
        (if (`/Game/PuzzelContent/Blueprints/CompletedSlabs/CombinedSlab.TileActive` _ascombined_slab)
          (if (not (`KismetArrayLibrary.Array_Contains` _currentanswer _array_index)) :!label _label
            (`KismetArrayLibrary.Array_Add` _currentanswer _array_index))
          (for _ (`self.AnswerKey`)
            (if (== (`KismetArrayLibrary.Array_Length` (`self.AnswerKey`)) (`KismetArrayLibrary.Array_Length` (`self.CurrentAnswer`)))
              (for (_array_element_2 _array_index_2) (`self.AnswerKey`)
                (if (== (`|GetArrayItem` (`self.CurrentAnswer`) _array_index_2) _array_element_2)
                  (if (== (`KismetArrayLibrary.Array_LastIndex` (`self.AnswerKey`)) _array_index_2)
                    (set `self.GameWon` true))))))
          (else
            (if (`KismetArrayLibrary.Array_Contains` _currentanswer_2 _array_index) :!label _label_2
              (`KismetArrayLibrary.Array_RemoveItem` _currentanswer_2 _array_index)))))
      (:`CastFailed`
        (bind _asred_puzzle_piece (cast `/Game/PuzzelContent/Blueprints/CompletedSlabs/RedPuzzlePiece` _array_element)
          (:`then`
            (if (`/Game/PuzzelContent/Blueprints/CompletedSlabs/RedPuzzlePiece.TileActive` _asred_puzzle_piece)
              (goto _label)
              (else
                (goto _label_2))))
          (:`CastFailed`
            (bind _asblue_puzzle_piece (cast `/Game/PuzzelContent/Blueprints/CompletedSlabs/BluePuzzlePiece` _array_element))
            (if (`/Game/PuzzelContent/Blueprints/CompletedSlabs/BluePuzzlePiece.TileActive` _asblue_puzzle_piece)
              (goto _label)
              (else
                (goto _label_2)))))))))

(fn `GenerateBoard`
  (bind _returnvalue (`SceneComponent.K2_GetComponentToWorld` (`self.DefaultSceneRoot`)))
  (bind _returnvalue_2 (`SceneComponent.K2_GetComponentToWorld` (`self.DefaultSceneRoot`)))
  (bind _returnvalue_3 (`SceneComponent.K2_GetComponentToWorld` (`self.DefaultSceneRoot`)))
  (for _index (range 5)
    (for _index_2 (range (+ (`self.GridSize`) 1))
      (switch `int` (`|GetArrayItem` (`self.GridTiles`) (`self.CurrentPlaceInTile`))
        (:`0`
          (bind _returnvalue_4 (`KismetMathLibrary.Conv_IntToDouble` (* _index_2 50)))
          (bind _returnvalue_5 (`KismetMathLibrary.Conv_IntToDouble` (* _index 50)))
          (bind _returnvalue_6 (`|SpawnActorFromClass` "/Game/PuzzelContent/Blueprints/CompletedSlabs/CombinedSlab.CombinedSlab_C" (`KismetMathLibrary.MakeTransform` (`KismetMathLibrary.MakeVector` (+ (+ (.x (.location _returnvalue_2)) _returnvalue_4) -250.0) (+ (.y (.location _returnvalue_2)) _returnvalue_5) (.z (.location _returnvalue_2)))) "AlwaysSpawn" "OverrideRootScale" null null))
          (bind _output_get (set `self.TileReferences` (`self.TileReferences`)))
          (`KismetArrayLibrary.Array_Add` _output_get _returnvalue_6)
          (`/Engine/EditorBlueprintResources/StandardMacros.IncrementInt` (`self.CurrentPlaceInTile`)))
        (:`1`
          (bind _returnvalue_7 (`|SpawnActorFromClass` "/Game/PuzzelContent/Blueprints/CompletedSlabs/RedPuzzlePiece.RedPuzzlePiece_C" (`KismetMathLibrary.MakeTransform` (`KismetMathLibrary.MakeVector` (+ (+ (.x (.location _returnvalue_3)) _returnvalue_4) -250.0) (+ (.y (.location _returnvalue_3)) _returnvalue_5) (.z (.location _returnvalue_3)))) "AlwaysSpawn" "OverrideRootScale" null null))
          (bind _output_get_2 (set `self.TileReferences` (`self.TileReferences`)))
          (`KismetArrayLibrary.Array_Add` _output_get_2 _returnvalue_7)
          (`/Engine/EditorBlueprintResources/StandardMacros.IncrementInt` (`self.CurrentPlaceInTile`)))
        (:`2`
          (bind _returnvalue_8 (`|SpawnActorFromClass` "/Game/PuzzelContent/Blueprints/CompletedSlabs/BluePuzzlePiece.BluePuzzlePiece_C" (`KismetMathLibrary.MakeTransform` (`KismetMathLibrary.MakeVector` (+ (+ (.x (.location _returnvalue)) _returnvalue_4) -250.0) (+ (.y (.location _returnvalue)) _returnvalue_5) (.z (.location _returnvalue)))) "AlwaysSpawn" "OverrideRootScale" null null))
          (bind _output_get_3 (set `self.TileReferences` (`self.TileReferences`)))
          (`KismetArrayLibrary.Array_Add` _output_get_3 _returnvalue_8)
          (`/Engine/EditorBlueprintResources/StandardMacros.IncrementInt` (`self.CurrentPlaceInTile`)))))))

(fn `SortCurrentAnwers`
  (locals (N :type Integer) (i :type Integer) (j :type Integer))
  ;[1 1 1] This function sorts them from smallest to largest. With index 0 Being the smallest. (Bubble Sort)
  (set `local.N` (`KismetArrayLibrary.Array_LastIndex` (`self.CurrentAnswer`)))
  (for _index (range (`local.N`))
    (set `local.i` _index)
    (for _index_2 (range (+ (- (`local.N`) 1 (`local.i`)) 1))
      (set `local.j` _index_2)
      (if (> (`|GetArrayItem` (`self.CurrentAnswer`) (`local.j`)) (`|GetArrayItem` (`self.CurrentAnswer`) (+ (`local.j`) 1)))
        (`KismetArrayLibrary.Array_Swap` (`self.CurrentAnswer`) (`local.j`) (+ (`local.j`) 1)))))
  (return))

(fn `UserConstructionScript`)